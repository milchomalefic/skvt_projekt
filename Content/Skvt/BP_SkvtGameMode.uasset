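; Game mode for the Skvt game that moves player control to a surviving character after a death.
; On BeginPlay it caches player 0's BP_SkvtPlayerController.
; AfterDeath has that controller possess the result of FIndNextCharacter, if valid.
; FIndNextCharacter scans all BP_SkvtBaseChar actors and returns the first one that is not dead.
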(event Custom|AfterDeath
  (bind _next_pawn (CallFunction|FIndNextCharacter))
  (Utilities|IsValid _next_pawn
    (:Is%20Valid
      (Pawn|Possess (Variables|Default|GetControllerRef) _next_pawn))))

(event EventBeginPlay
  (bind _asbp_skvt_player_controller (Utilities|Casting|CastToBP_SkvtPlayerController (Game|GetPlayerController 0)))
  (Variables|Default|SetControllerRef _asbp_skvt_player_controller))

(fn ConstructionScript)

(fn FIndNextCharacter
  (bind _outactors (Actor|GetAllActorsOfClass "/Game/Skvt/Characters/BP_SkvtBaseChar.BP_SkvtBaseChar_C"))
  (for _array_element _outactors
    (if (not (Default|IsDead _array_element))
      (return _array_element))))