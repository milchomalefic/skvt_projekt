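; Blueprint function library with a helper that finds the nearest actor to a target location among the actors overlapping a given target.
; It loops over the overlaps, keeps the one with the smallest vector distance to that location, and returns that actor and its distance.
; The overlap query filters on the base Actor class, so the Class input is unused despite the function's name.
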(fn FIndNearestActorOfClass
  (params (Class :type Actor%20Class%20Reference) (TargetLocation :type Vector) (Target :type Actor%20Object%20Reference))
  (for _array_element (Collision|GetOverlappingActors Target "/Script/Engine.Actor" :!class /Script/Engine.Actor)
    (if (< (Math|Vector|Distance(Vector) (Transformation|GetActorLocation _array_element) TargetLocation) (LocalVariables|GetLoc_NearestDistance))
      (LocalVariables|SetLoc_NearestDistance (Math|Vector|Distance(Vector) (Transformation|GetActorLocation _array_element) TargetLocation))
      (LocalVariables|SetLoc_NearestActor _array_element)))
  (return (LocalVariables|GetLoc_NearestActor) (LocalVariables|GetLoc_NearestDistance)))