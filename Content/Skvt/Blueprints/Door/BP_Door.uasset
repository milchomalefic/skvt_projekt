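; BP_Door is an interactable door that swings open and closed on its yaw axis.
; Interact uses a FlipFlop to play or reverse a timeline that lerps the door mesh rotation and switches the prompt text between Open and Close.
; ShowInteraction creates a WBP_Interaction prompt and turns on the mesh's custom depth rendering, and HideInteraction removes both.
; The timeline update also pushes the current text to the widget.
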(event EventBeginPlay)

(event Collision|EventActorBeginOverlap
  (params (OtherActor :type Actor%20Object%20Reference)))

(event EventTick
  (params (DeltaSeconds :type Float%20%28single-precision%29)))

(event EventInteract
  ;[0.1302 0.04336 0.06431] OpenDoor
  (Utilities|FlowControl|FlipFlop
    (:A
      (Variables|Default|SetInteractionText "Close")
      (bind _doorrotation (Timeline|Timeline Play)
        (:Update
          (Transformation|SetRelativeRotation (Variables|Default|GetSM_Door) (Math|Rotator|MakeRotator 0.0 0.0 (Math|Float|Lerp 0.0 1e+02 _doorrotation)) false false)
          (Class|BPIInteraction|SetInteraction(Message) (Variables|Default|GetInteractionWidget) (Variables|Default|GetInteractionText)))))
    (:B
      (Variables|Default|SetInteractionText "Open")
      (Timeline|Timeline Reverse))))

(event EventShowInteraction
  (bind _returnvalue (UserInterface|CreateWidget "/Game/Skvt/UI/Widgets/Interactions/WBP_Interaction.WBP_Interaction_C"))
  (bind _output_get (Variables|Default|SetInteractionWidget _returnvalue))
  (UserInterface|Viewport|AddtoViewport _output_get 0)
  (Class|BPIInteraction|SetInteraction(Message) _output_get (Variables|Default|GetInteractionText))
  (Rendering|SetRenderCustomDepth (Variables|Default|GetSM_Door) true))

(event EventHideInteraction
  (bind _interactionwidget (Variables|Default|GetInteractionWidget))
  (Utilities|IsValid _interactionwidget
    (:Is%20Valid
      (Widget|RemovefromParent _interactionwidget)
      (Rendering|SetRenderCustomDepth (Variables|Default|GetSM_Door) false))))

(fn ConstructionScript)