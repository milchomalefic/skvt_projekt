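; Platform actor that sends turn-off and break messages to nearby devices when any actor overlaps it.
; GetNearbyDevices runs a Pawn-only sphere overlap around the player character rather than the platform, and draws a debug sphere of the search area.
; The returned actors receive both messages in sequence; loops over Lights and Devices are left unconnected.
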(event EventBeginPlay)

(event Collision|EventActorBeginOverlap
  (params (OtherActor :type Actor%20Object%20Reference))
  (bind _nearbydevices (CallFunction|GetNearbyDevices))
  (Class|BPIElectricDevices|TurnOffDevices(Message) _nearbydevices)
  (Class|BPIElectricDevices|BreakDevices(Message) _nearbydevices))

(event EventTick
  (params (DeltaSeconds :type Float%20%28single-precision%29)))

(fn ConstructionScript)

(fn GetNearbyDevices
  (bind _returnvalue (Game|GetPlayerCharacter 0))
  (bind _returnvalue_2 (Transformation|GetActorLocation _returnvalue))
  (Rendering|Debug|DrawDebugSphere _returnvalue_2 5e+02 24 "(R=1.000000,G=1.000000,B=1.000000,A=1.000000)" 2.0 1.0)
  (bind _outactors (Collision|SphereOverlapActors _returnvalue_2 5e+02 (Utilities|Array|MakeArray "ObjectTypeQuery3") 0))
  (return _outactors))