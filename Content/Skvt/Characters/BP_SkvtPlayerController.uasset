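; Player controller for Skvt that sets up input and HUD, pawn swapping, and the in-game menu.
; On BeginPlay it adds the PMI_SkvtMapping Enhanced Input config and creates the player HUD, whose health bar can be pointed at a given component.
; The swap input possesses the next Pawn found in the level, wrapping to the first.
; The menu input toggles WBP_MainMenu along with pause, cursor and input mode.
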(event Input|EnhancedActionEvents|EnhancedInputActionIA_Swap
  (params (ActionValue :type Boolean) (ElapsedSeconds :type Float%20%28double-precision%29) (TriggeredSeconds :type Float%20%28double-precision%29) (InputAction :type Input%20Action%20Object%20Reference :default "/Game/Skvt/Characters/Input/Actions/IA_Swap.IA_Swap"))
  ;[0.1146 0.1146 0.1146] Swap Characters
  (:Triggered
    (bind _outactors (Actor|GetAllActorsOfClass "/Script/Engine.Pawn"))
    (if (Utilities|Array|IsValidIndex _outactors (+ (Utilities|Array|FindItem _outactors (Pawn|GetControlledPawn)) 1))
      (Pawn|Possess (Utilities|Array|Get(acopy) _outactors (+ (Utilities|Array|FindItem _outactors (Pawn|GetControlledPawn)) 1)))
      (else
        (Pawn|Possess (Utilities|Array|Get(acopy) _outactors))))))

(event Input|EnhancedActionEvents|EnhancedInputActionIA_OpenMenu
  (params (ActionValue :type Boolean) (ElapsedSeconds :type Float%20%28double-precision%29) (TriggeredSeconds :type Float%20%28double-precision%29) (InputAction :type Input%20Action%20Object%20Reference :default "/Game/Skvt/Characters/Input/Actions/IA_OpenMenu.IA_OpenMenu"))
  ;[0.2865 0.1569 0.2682] Ingame Menu
  (:Triggered
    (Utilities|IsValid (Variables|Default|GetGameMenu)
      (:Is%20Valid
        (if (Widget|IsVisible (Variables|Default|GetGameMenu))
          (Input|SetInputModeGameOnly self false)
          (Variables|Default|SetbShowMouseCursor false)
          (Game|SetGamePaused false)
          (Widget|RemovefromParent (Variables|Default|GetGameMenu))
          (else
            (bind _returnvalue (UserInterface|CreateWidget "/Game/Skvt/UI/Widgets/Menu/WBP_MainMenu.WBP_MainMenu_C" self :!label _label))
            (bind _output_get (Variables|Default|SetGameMenu _returnvalue))
            (UserInterface|Viewport|AddtoViewport _output_get 0)
            (Input|SetInputModeGameandUI self 0 "DoNotLock" true false)
            (Variables|Default|SetbShowMouseCursor true)
            (Game|SetGamePaused true))))
      (:Is%20Not%20Valid
        (goto _label)))))

(event EventBeginPlay
  (bind _self self)
  (bind _returnvalue (PlayerController|LocalPlayerSubsystems|GetEnhancedInputLocalPlayerSubsystem _self))
  ;[0.07812 0.07202 0.01398] Add PMI Mapping
  (Utilities|IsValid _returnvalue
    (:Is%20Valid
      (Class|EnhancedInputSubsystemInterface|AddPlayerMappableConfig _returnvalue "/Game/Skvt/Characters/Input/PMI_SkvtMapping.PMI_SkvtMapping" "(bIgnoreAllPressedKeysUntilRelease=True,bForceImmediately=False)")
      ;[0.1719 0.04771 0.09886] Create HUD
      (CallFunction|CreatePlayerHUD))))

(fn ConstructionScript)

(fn CreatePlayerHUD
  (bind _returnvalue (UserInterface|CreateWidget "/Game/Skvt/UI/PlayerHUD/WBP_PlayerHUD.WBP_PlayerHUD_C"))
  (bind _output_get (Variables|Default|SetPlayerHUD _returnvalue))
  (UserInterface|Viewport|AddtoViewport _output_get 0))

(fn UpdateHealthComponentHUD
  (params (NewComponent :type Skvt%20Health%20Component%20Object%20Reference))
  (bind _playerhud (Variables|Default|GetPlayerHUD))
  (Utilities|IsValid _playerhud
    (:Is%20Valid
      (Default|UpdateHealthBar _playerhud NewComponent))))