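; Actor component that provides helper functions to show and hide an interaction prompt with a mesh highlight.
; ShowInteraction creates a WBP_Interaction widget, adds it to the viewport, sets its message, enables custom depth on the given mesh, and returns the widget.
; HideInteraction removes that widget and disables custom depth, touching the mesh only when the widget is valid.
; The component holds no event logic, so callers supply the mesh and keep the widget reference.
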(event EventBeginPlay)

(event EventTick
  (params (DeltaSeconds :type Float%20%28single-precision%29)))

(fn ShowInteraction
  (params (OutlineStaticMesh :type Static%20Mesh%20Component%20Object%20Reference) (InteractionText :type Text))
  (bind _returnvalue (UserInterface|CreateWidget "/Game/Skvt/UI/Widgets/Interactions/WBP_Interaction.WBP_Interaction_C"))
  (UserInterface|Viewport|AddtoViewport _returnvalue 0)
  (Class|BPIInteraction|SetInteraction(Message) _returnvalue InteractionText)
  (Utilities|IsValid OutlineStaticMesh
    (:Is%20Valid
      (Rendering|SetRenderCustomDepth OutlineStaticMesh true)
      (return _returnvalue))
    (:Is%20Not%20Valid
      (return _returnvalue))))

(fn HideInteraction
  (params (InteractionWidget :type WBP%20Interaction%20Object%20Reference) (OutlineStaticMesh :type Static%20Mesh%20Component%20Object%20Reference))
  (Utilities|IsValid InteractionWidget
    (:Is%20Valid
      (Widget|RemovefromParent InteractionWidget)
      (Utilities|IsValid OutlineStaticMesh
        (:Is%20Valid
          (Rendering|SetRenderCustomDepth OutlineStaticMesh false))))))